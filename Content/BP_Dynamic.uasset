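; Actor that shows a texture-displaced dynamic sphere or an undisplaced plane, using Geometry Script meshes.
; BeginPlay caches both shapes from static mesh assets and starts a looping timer.
; Each tick of that timer copies the clean sphere or plane, chosen by DepthSimu, into a working mesh on the component.
; The sphere is then displaced by DisplacementMap and its normals recomputed, so displacement never accumulates.
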(event `self.ReceiveBeginPlay`
  ;[1 1 1] Creation of Dynamic Meshes
  (`KismetSystemLibrary.K2_SetTimerDelegate` (delegate `UpdateDepth`) (`self.Loop Time`) true)
  ;;[1 1 1] Dynamic Sphere
  (bind _returnvalue (`|GenericCreateObject` "/Script/GeometryFramework.DynamicMesh"))
  (bind _output_get (set `self.Sphere Msh` _returnvalue))
  (bind _returnvalue_2 (`GeometryScriptLibrary_StaticMeshFunctions.CopyMeshFromStaticMesh` (`self.Custom Sphere Shape`) _output_get (struct) (struct) null)
    (:`Success`
      (bind _returnvalue_3 (`|GenericCreateObject` "/Script/GeometryFramework.DynamicMesh"))
      (bind _output_get_2 (set `self.Temp` _returnvalue_3))
      (`GeometryScriptLibrary_MeshDecompositionFunctions.CopyMeshToMesh` _returnvalue_2 _output_get_2 null)
      (`DynamicMeshComponent.SetDynamicMesh` (`self.DynamicMeshComponent`) (`self.Temp`))
      ;;[1 1 1] Dynamic Plane
      (bind _returnvalue_4 (`|GenericCreateObject` "/Script/GeometryFramework.DynamicMesh"))
      (bind _output_get_3 (set `self.Plane Msh` _returnvalue_4))
      (`GeometryScriptLibrary_StaticMeshFunctions.CopyMeshFromStaticMesh` (`self.Custom Plane Shape`) _output_get_3 (struct) (struct) null))))

(event `UpdateDepth`
  ;[1 1 1] Displacement
  (if (`self.DepthSimu`)
    (`GeometryScriptLibrary_MeshDecompositionFunctions.CopyMeshToMesh` (`self.Sphere Msh`) (`self.Temp`) null)
    (else
      (`GeometryScriptLibrary_MeshDecompositionFunctions.CopyMeshToMesh` (`self.Plane Msh`) (`self.Temp`) null)))
  (`DynamicMeshComponent.SetDynamicMesh` (`self.DynamicMeshComponent`) (`self.Temp`))
  (if (`self.DepthSimu`)
    (bind _returnvalue (`BaseDynamicMeshComponent.GetDynamicMesh` (`self.DynamicMeshComponent`)))
    (bind _returnvalue_2 (`MeshUtils.DisplaceMeshFromTexture` _returnvalue (`self.Displacement Map`) (`self.Magnitude`) (`self.Neutral Gray`)))
    (`GeometryScriptLibrary_MeshNormalsFunctions.RecomputeNormals` _returnvalue_2 (struct) null)))

(fn `UserConstructionScript`)